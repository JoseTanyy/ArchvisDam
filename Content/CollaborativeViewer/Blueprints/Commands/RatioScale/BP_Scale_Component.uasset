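; Command component for the Collaborative Viewer that lets the user change the world scale ratio through the pawn's SetWorldScale.
; After pawn spawn it creates a "Scale 1:1" button with a slider widget as an option.
; It also reuses or creates a ratio toolbar in the desktop UI's middle toolbar.
; Slider changes and toolbar commits both set the world ratio and update the other widget to keep them in sync.
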(event `self.ReceiveBeginPlay`
  (bind _returnvalue (`|CreateWidget` "/Game/CollaborativeViewer/Blueprints/Commands/RatioScale/UMG/Slider.Slider_C"))
  (set `self.Slider` _returnvalue))

(event `AddRatioToolBar`
  (bind _foundwidgets (`WidgetBlueprintLibrary.GetAllWidgetsOfClass` "/Game/CollaborativeViewer/Blueprints/Commands/RatioScale/UMG/ScaleRatioToolBar.ScaleRatioToolBar_C" false))
  (if (> (`KismetArrayLibrary.Array_Length` _foundwidgets) 0)
    (set `self.ScaleRationToolBar` (`|GetArrayItem` _foundwidgets))
    (else
      (bind _asbp_collab_v_player_controller (cast `/Game/CollaborativeViewer/Blueprints/PlayerController/BP_Collab_V_PlayerController` (`GameplayStatics.GetPlayerController` 0)))
      (bind _returnvalue (`|CreateWidget` "/Game/CollaborativeViewer/Blueprints/Commands/RatioScale/UMG/ScaleRatioToolBar.ScaleRatioToolBar_C"))
      (bind _output_get (set `self.ScaleRationToolBar` _returnvalue))
      (`PanelWidget.AddChild` (`/Game/CollaborativeViewer/UMG/GameMenu/Destop_UI.MiddleToolBar` (`/Game/CollaborativeViewer/Blueprints/PlayerController/BP_Collab_V_PlayerController.Desktop_UI` _asbp_collab_v_player_controller)) _output_get))))

(event `self.ExecuteAfterSpawnPawn`
  (bind _commandbutton (`self.CommandButton`))
  (bind _slider (`self.Slider`))
  ;[0 1 0.1488] BeginPLay
  (`parent.ExecuteAfterSpawnPawn`)
  (set `self.Icon` "/Game/CollaborativeViewer/Blueprints/Commands/RatioScale/RatioScale.RatioScale")
  (set `self.Name` (`KismetTextLibrary.Conv_StringToText` (`KismetStringLibrary.Concat_StrStr` "Scale  " (`KismetStringLibrary.Conv_IntToString` 1) " : " (`KismetStringLibrary.Conv_IntToString` 1))))
  (`self.CreateActivateButton`)
  (set `/Game/CollaborativeViewer/Blueprints/Commands/RatioScale/UMG/Slider.CommandButton` _commandbutton _slider)
  (`KismetArrayLibrary.Array_Add` (`/Game/CollaborativeViewer/UMG/GameMenu/CommandButton.Options` _commandbutton) _slider)
  (add `/Game/CollaborativeViewer/Blueprints/Commands/RatioScale/UMG/Slider.ChangedScale` _slider (delegate `SliderScaleChanged`))
  (`self.AddRatioToolBar`)
  (`self.BindCommited`)
  (`/Game/CollaborativeViewer/Blueprints/Commands/RatioScale/UMG/ScaleRatioToolBar.SetAtSpawn` (`self.ScaleRationToolBar`)))

(event `SliderScaleChanged`
  (params (Dividend :type Integer) (Divisor :type Integer))
  (`self.SetWorldRatio` Dividend Divisor)
  (`/Game/CollaborativeViewer/Blueprints/Commands/RatioScale/UMG/ScaleRatioToolBar.SetRatioToolBarValues` (`self.ScaleRationToolBar`) Dividend Divisor))

(event `SetWorldRatio`
  (params (Dividend :type Integer) (Divisor :type Integer))
  ;[0.2555 0.7775 1] Setup Option Buttons
  (`/Game/CollaborativeViewer/Blueprints/Pawn/BP_BasePawn.SetWorldScale` (`self.BasePawn`) Dividend Divisor))

(event `BindCommited`
  (add `/Game/CollaborativeViewer/Blueprints/Commands/RatioScale/UMG/ScaleRatioToolBar.SizeCommited` (`self.ScaleRationToolBar`) (delegate `ToolBarRatioChanged`)))

(event `ToolBarRatioChanged`
  (params (Dividend :type Integer) (Divisor :type Integer))
  (`self.SetWorldRatio` Dividend Divisor)
  (`/Game/CollaborativeViewer/Blueprints/Commands/RatioScale/UMG/Slider.SetRatioSliderValues` (`self.Slider`) Dividend Divisor))